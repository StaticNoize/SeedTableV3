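; Seed table placeable that acts as a crafting station able to use artisan thralls.
; It exposes its ThrallInventory through GetArtisanThrallInventory and always reports that thralls can be used.
; BeginPlay and construction defer to the parent, while EndPlay also unbinds all SOSWorkAlchemy state-change events.
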(event `self.ReceiveBeginPlay`
  (`parent.ReceiveBeginPlay`))

(event `self.ReceiveEndPlay`
  (params (EndPlayReason :type "EEndPlayReason Enum" :default "Destroyed"))
  (`parent.ReceiveEndPlay` EndPlayReason)
  (clear `SmartObjectSlotComponent.OnStateChanged` (`self.SOS_Work_Alchemy`)))

(fn `CanStationUseThralls`
  (returns (ReturnValue :type Boolean))
  (return true))

(fn `GetArtisanThrallInventory`
  (returns (ReturnValue :type "ItemInventory Object Reference"))
  (return (`self.ThrallInventory`)))

(fn `UserConstructionScript`
  (`parent.UserConstructionScript`))