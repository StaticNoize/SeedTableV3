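; Usable potion item that grants the Emberlight seed table feat to the character who drinks it.
; On use, it force-learns the feat through the progression system, then shows a local notification on listen servers and clients, skipping dedicated servers.
; The parent use logic runs last to work around a bug with the final item in a stack.
; It is always usable and its journey update records lotus potion drinking events server-side.
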(event `self.OnUseItem`
  (params (invokingCharacter :type "ConanCharacter Object Reference") (ownerPlayer :type "ConanCharacter Object Reference"))
  (bind _returnvalue (`ConanCharacter.GetProgressionSystem` invokingCharacter))
  (`ProgressionSystem.ServerForceLearnFeat` _returnvalue 4647199 false)
  ;[1 0.6413 0.1882] Notification
  (if (`/Game/Systems/MiscFunctions.IsListenServer` self)
    (message `/Game/Characters/HUDNotification_Interface.NotificationText` (`GameplayStatics.GetPlayerController` 0) "Seed Table: Emberlight Feat Added" true :!label _label)
    (elif (`KismetSystemLibrary.IsServer`)
      _
      (else
        (goto _label))))
  ;[1 1 1] Called at the end to fix bug where item not working if it is the last in the stack
  (`parent.OnUseItem` invokingCharacter null))

(fn `CanUseItem`
  (params (invokingCharacter :type "ConanCharacter Object Reference"))
  (returns (ReturnValue :type Boolean))
  (return true))

(fn `UpdateJourneyEvent`
  (params (InvokingCharacter :type "ConanCharacter Object Reference"))
  (if (`KismetSystemLibrary.IsServer`)
    (bind _asbase_player_char_interface (cast `/Game/Systems/Interfaces/BasePlayerCharInterface` InvokingCharacter))
    (`/Game/Systems/Interfaces/BasePlayerCharInterface.AddJourneyEventInterfaceCall` _asbase_player_char_interface "DrinkLotusPotion")
    (`/Game/Systems/Interfaces/BasePlayerCharInterface.AddJourneyEventInterfaceCall` _asbase_player_char_interface "Siptah_DrinkLotusPotion")))