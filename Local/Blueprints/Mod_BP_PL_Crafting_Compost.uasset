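; Placeable compost crafting station that periodically generates an item while its inventory holds either of two fertilizer items, without consuming them.
; A looping server timer counts fertilizer and adds the output if below one stack's maximum and space allows.
; The server stops the timer when UpdateMesh finds the inventory at MaxItems.
; An inventory client monitor and inventory signals toggle the mesh to show whether fertilizer is present.
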(event `self.ReceiveBeginPlay`
  (bind _placeableinventory (`self.PlaceableInventory`))
  (`parent.ReceiveBeginPlay`)
  (bind _returnvalue (`|GenericCreateObject` "/Script/ConanSandbox.ItemInventoryClientMonitor" self))
  (bind _output_get (set `self.InventoryMonitor` _returnvalue))
  (`ItemInventoryClientMonitor.SetInventory` _output_get _placeableinventory)
  (add `ItemInventory.SignalInventoryRecivedOnClient` _placeableinventory (delegate `UpdateMesh`))
  (if (`KismetSystemLibrary.IsServer`)
    (if (not (`self.IsABrush`))
      (bind _returnvalue_2 (`KismetSystemLibrary.K2_SetTimerDelegate` (delegate `Tick`) (* (`self.Tick Time`) (`self.Tick modifier`)) true))
      (set `self.TimerHandle` _returnvalue_2))))

(event `Tick`
  (`self.CountFertilizer`)
  (if (not (== (`self.ResourceCount`) 0))
    (switch `int` (`KismetMathLibrary.RandomInteger` 1)
      (:`0`
        (bind _returnvalue (`|GetDataTableRow` "/Game/Items/ItemTable.ItemTable" "13012")
          (:`then`
            (if (< (`ItemInventory.GetResourceCount` (`self.PlaceableInventory`) 13012 false) (`.MaxStackSize` (break `ItemTableRow` _returnvalue)))
              (`self.SpawnResultItem` 13012))))))))

(event `UpdateMesh`
  (bind _staticmesh1 (`self.StaticMesh1`))
  (`|ExecutionSequence`
    (:`then_0`
      (if (`KismetSystemLibrary.IsServer`)
        (if (== (`ItemInventory.GetItemCount` (`self.PlaceableInventory`)) (`self.Max Items`))
          (`KismetSystemLibrary.K2_ClearAndInvalidateTimerHandle` (`self.TimerHandle`))
          (else
            (bind _returnvalue (`KismetSystemLibrary.K2_SetTimerDelegate` (delegate `Tick`) (* (`self.Tick Time`) (`self.Tick modifier`)) true))
            (set `self.TimerHandle` _returnvalue)))))
    (:`then_1`
      (`SceneComponent.SetVisibility` _staticmesh1 false false :!label _label)
      (set `self.ResourceCount` 0)
      (`self.CountFertilizer`)
      (if (> (`self.ResourceCount`) 0)
        (`SceneComponent.SetVisibility` _staticmesh1 true false)))))

(event `self.PlaceableInventory.SignalItemRemoved`
  (params (index :type Integer) (item :type "GameItem Object Reference") (dstInventory :type "ItemInventory Object Reference") (dstIndex :type Integer))
  (goto _label))

(event `self.PlaceableInventory.SignalItemAdded`
  (params (index :type Integer) (item :type "GameItem Object Reference") (srcInventory :type "ItemInventory Object Reference") (srcIndex :type Integer))
  (goto _label))

(fn `CountFertilizer`
  (set `self.ResourceCount` (+ (`ItemInventory.GetResourceCount` (`self.PlaceableInventory`) 11076 false) (`self.ResourceCount`)))
  (set `self.ResourceCount` (+ (`ItemInventory.GetResourceCount` (`self.PlaceableInventory`) 11077 false) (`self.ResourceCount`))))

(fn `GetArtisanThrallInventory`
  (returns (ReturnValue :type "ItemInventory Object Reference"))
  (return null))

(fn `SpawnResultItem`
  (params (`TemplateID to Spawn1` :type Integer))
  (locals (`TemplateID to Spawn` :type Integer))
  (bind _returnvalue (`ItemInventory.FindItemByTemplateID` (`self.PlaceableInventory`) (`local.TemplateID to Spawn`) (`self.CurrentInventoryIndex`)))
  (bind _returnvalue_2 (`ItemInventory.GetItem` (`self.PlaceableInventory`) _returnvalue))
  (set `local.TemplateID to Spawn` `TemplateID to Spawn1`)
  (if (not (< (`ItemInventory.GetPopulatedItemCount` (`self.PlaceableInventory`) 0 -1) (`ItemInventory.MaxItemCount` (`self.PlaceableInventory`))))
    (set `self.CurrentInventoryIndex` 0)
    (if (!= _returnvalue -1) :!label _label
      (if (< (`GameItem.GetIntStat` _returnvalue_2 "StackSize") (`GameItem.GetIntStat` _returnvalue_2 "MaxStackSize"))
        _
        (else
          (set `self.CurrentInventoryIndex` (+ (`self.CurrentInventoryIndex`) 1))
          (goto _label)))
      (else
        (return))))
  (`ItemInventory.AddItemTemplate` (`self.PlaceableInventory`) (`local.TemplateID to Spawn`) -1 "None" 1 false 1.0 -1.0)
  (return))

(fn `UserConstructionScript`
  (`parent.UserConstructionScript`))